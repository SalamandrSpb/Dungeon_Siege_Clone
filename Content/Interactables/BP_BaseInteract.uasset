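; Base interactable actor for items the player picks up with a mouse click.
; Cursor hover over its Sphere toggles custom depth rendering on the Item component, typically used for highlighting.
; A click gets a reference through RefPlayerMessage on the player pawn, calls Pickup with the actor's location, and destroys the actor if that succeeds.
; Its own RefPlayer function and construction script are empty.
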(event `self.Sphere.OnBeginCursorOver`
  (params (TouchedComponent :type "PrimitiveComponent Object Reference"))
  (`PrimitiveComponent.SetRenderCustomDepth` (`self.Item`) true))

(event `self.Sphere.OnEndCursorOver`
  (params (TouchedComponent :type "PrimitiveComponent Object Reference"))
  (`PrimitiveComponent.SetRenderCustomDepth` (`self.Item`) false))

(event `self.Sphere.OnClicked`
  (params (TouchedComponent :type "PrimitiveComponent Object Reference") (ButtonPressed :type "Key Structure"))
  (bind _player (message `/Game/Interactables/BPI_Interact.RefPlayer` (`GameplayStatics.GetPlayerPawn` 0)))
  (bind _canpickup (`/Game/Blueprints/BP_Player.Pickup` _player (`self.K2_GetActorLocation`)))
  (if _canpickup
    (`self.K2_DestroyActor`)))

(fn `RefPlayer`
  (returns (Player :type "/Game/Blueprints/BP_Player Object Reference"))
  (return null))

(fn `UserConstructionScript`)