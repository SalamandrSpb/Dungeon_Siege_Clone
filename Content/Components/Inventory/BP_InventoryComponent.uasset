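; Inventory component that shows and hides the inventory widget on screen.
; ShowInventory sets the open flag, constructs a new WBP_Inventory with the first player's pawn as outer, stores it and adds it to the viewport.
; HideInventory removes the stored widget from its parent and clears the flag, only if that widget is valid.
; It holds no item logic, and its BeginPlay and Tick events are unused.
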(fn `HideInventory`
  (`/Engine/EditorBlueprintResources/StandardMacros.IsValid` (`self.WBPInventory`)
    (:`Is Valid`
      (`Widget.RemoveFromParent` (`self.WBPInventory`))
      (set `self.IsInvetoryOpen` false))))

(fn `ShowInventory`
  (set `self.IsInvetoryOpen` true)
  (bind _returnvalue (`|GenericCreateObject` "/Game/Components/Inventory/WBP_Inventory.WBP_Inventory_C" (`GameplayStatics.GetPlayerPawn` 0)))
  (bind _output_get (set `self.WBPInventory` _returnvalue))
  (`UserWidget.AddToViewport` _output_get 0))