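; BP_Player is the player Blueprint, handling third-person camera control and switching between character animation sets.
; Look and turn input rotate the view only while the UnlockCamera action is held.
; The zoom axis adjusts the spring arm length by a step, clamped to a fixed range.
; Number keys swap the mesh's Animation Blueprint between player, swordsman, wizard and archer classes at runtime.
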(event `InputAxis|LookUp`
  (params (AxisValue :type "Float (single-precision)"))
  ;[1 1 1] Управление камерой
  (if (`self.UnlockCamera`)
    (`self.AddControllerPitchInput` AxisValue)))

(event `InputAxis|Turn`
  (params (AxisValue :type "Float (single-precision)"))
  ;[1 1 1] Управление камерой
  (if (`self.UnlockCamera`)
    (`self.AddControllerYawInput` AxisValue)))

(event `InputAction|UnlockCamera`
  (params (Key :type "Key Structure"))
  ;[1 1 1] Можно повернуть камеру или нет?
  (:`Pressed`
    (set `self.UnlockCamera` true))
  (:`Released`
    (set `self.UnlockCamera` false)))

(event `InputAxis|CameraZoom`
  (params (AxisValue :type "Float (single-precision)"))
  (bind _springarm (`self.SpringArm`))
  (set `SpringArmComponent.TargetArmLength` (`KismetMathLibrary.FClamp` (- (`SpringArmComponent.TargetArmLength` _springarm) (* AxisValue (`self.CameraZoomStep`))) 300.0 1000.0) _springarm))

(event `Key|One`
  (params (Key :type "Key Structure"))
  (:`Pressed`
    (`SkeletalMeshComponent.SetAnimInstanceClass` (`self.Mesh`) "/Game/Animations/ABP_Player.ABP_Player_C")))

(event `Key|Two`
  (params (Key :type "Key Structure"))
  (:`Pressed`
    (`SkeletalMeshComponent.SetAnimInstanceClass` (`self.Mesh`) "/Game/Animations/ABP_Swordsman.ABP_Swordsman_C")))

(event `Key|Three`
  (params (Key :type "Key Structure"))
  (:`Pressed`
    (`SkeletalMeshComponent.SetAnimInstanceClass` (`self.Mesh`) "/Game/Animations/ABP_Wizard.ABP_Wizard_C")))

(event `Key|Four`
  (params (Key :type "Key Structure"))
  (:`Pressed`
    (`SkeletalMeshComponent.SetAnimInstanceClass` (`self.Mesh`) "/Game/Animations/ABP_Archer.ABP_Archer_C")))

(fn `UserConstructionScript`)